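; Gameplay ability that zooms the FourTale character's camera for aiming while the input is held, acting only for the locally controlled player.
; Activation caches the CameraBoom and its current arm length, and input release reverses the zoom.
; Looping timers drive ZoomIn and ZoomOut, which lerp arm length through a shared Alpha, so reversals continue from the current blend.
; The ability ends once zoom-out completes.
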(event Custom|ChangeAiming
  (params (IsAiming :type Boolean))
  (bind _returnvalue (Utilities|Time|GetWorldDeltaSeconds))
  (CallFunction|ClearHandles)
  (if IsAiming
    (bind _returnvalue_2 (Utilities|Time|SetTimerbyEvent (EventDispatchers|CreateEvent :!event Zoomin) _returnvalue true true))
    (Variables|Default|SetZoomInTimerHandle _returnvalue_2)
    (else
      (bind _returnvalue_3 (Utilities|Time|SetTimerbyEvent (EventDispatchers|CreateEvent :!event ZoomOut) _returnvalue true true))
      (Variables|Default|SetZoomOutTimerHandle _returnvalue_3))))

(event Ability|EventActivateAbility
  (Pawn|IsLocallyControlled
    (:True
      (Variables|Default|GetCameraBoom
        (:then
          _)
        (:else
          (CallFunction|SetCameraBoom)))
      (CallFunction|SetDefaultArmLength)
      (CallFunction|ChangeAiming true)
      (Ability|Tasks|WaitInputRelease true
        (:OnRelease
          (CallFunction|ChangeAiming false))))))

(event Ability|EventOnEndAbility
  (params (bWasCancelled :type Boolean)))

(fn SetDefaultArmLength
  (Variables|Default|SetDefaultArmLenth (Variables|/Script/Engine.SpringArmComponent|GetTargetArmLength (Variables|Default|GetCameraBoom))))

(fn SetCameraBoom
  (bind _asbp_four_tale_character (Utilities|Casting|CastToBP_FourTaleCharacter (Ability|GetAvatarActorfromActorInfo)))
  (Variables|Default|SetCameraBoom (Variables|/Script/FourTaleTestProject.FourTaleCharacter|GetCameraBoom _asbp_four_tale_character)))

(fn ZoomOut
  (bind _cameraboom (Variables|Default|GetCameraBoom))
  (bind _output_get (Variables|Default|SetAlpha (- (Variables|Default|GetAlpha) (* (Utilities|Time|GetWorldDeltaSeconds) (Variables|Default|GetLengthChangeSpeed)))))
  (if (< _output_get 0.0)
    (Variables|Default|SetAlpha 0.0)
    (Variables|/Script/Engine.SpringArmComponent|SetTargetArmLength _cameraboom (Variables|Default|GetDefaultArmLenth))
    (Utilities|Time|ClearandInvalidateTimerbyHandle (Variables|Default|GetZoomOutTimerHandle))
    (Ability|EndAbility)
    (else
      (Variables|/Script/Engine.SpringArmComponent|SetTargetArmLength _cameraboom (Math|Float|Lerp (Variables|Default|GetDefaultArmLenth) (Variables|Default|GetAimArmLength) _output_get)))))

(fn Zoomin
  (bind _cameraboom (Variables|Default|GetCameraBoom))
  (bind _output_get (Variables|Default|SetAlpha (+ (Variables|Default|GetAlpha) (* (Utilities|Time|GetWorldDeltaSeconds) (Variables|Default|GetLengthChangeSpeed)))))
  (if (> _output_get 1.0)
    (Variables|Default|SetAlpha 1.0)
    (Variables|/Script/Engine.SpringArmComponent|SetTargetArmLength _cameraboom (Variables|Default|GetAimArmLength))
    (Utilities|Time|ClearandInvalidateTimerbyHandle (Variables|Default|GetZoomInTimerHandle))
    (else
      (Variables|/Script/Engine.SpringArmComponent|SetTargetArmLength _cameraboom (Math|Float|Lerp (Variables|Default|GetDefaultArmLenth) (Variables|Default|GetAimArmLength) _output_get)))))

(fn ClearHandles
  (Utilities|Time|ClearandInvalidateTimerbyHandle (Variables|Default|GetZoomInTimerHandle))
  (Utilities|Time|ClearandInvalidateTimerbyHandle (Variables|Default|GetZoomOutTimerHandle)))