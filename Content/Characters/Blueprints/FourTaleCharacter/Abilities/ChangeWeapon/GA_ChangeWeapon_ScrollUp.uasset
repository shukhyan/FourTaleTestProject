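; GA_ChangeWeapon_ScrollUp is a Gameplay Ability that switches the FourTale character's weapon in a scroll direction.
; On activation it uses the cached character, or casts the avatar actor to BP_FourTaleCharacter and caches it if invalid.
; It then unequips the weapon, changes the current weapon index using the IsScrollUp flag, equips the new weapon and ends the ability immediately.
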(event Ability|EventActivateAbility
  (Variables|FourTale|GetCharacter
    (:then
      _)
    (:else
      (bind _asbp_four_tale_character (Utilities|Casting|CastToBP_FourTaleCharacter (Ability|GetAvatarActorfromActorInfo)))
      (bind _output_get (Variables|FourTale|SetCharacter _asbp_four_tale_character))))
  (Class|FourTaleCharacter|UnequipWeapon _output_get)
  (Class|FourTaleCharacter|ChangeCurrentWeaponIndex (Variables|FourTale|GetCharacter) (Variables|FourTale|GetIsScrollUp))
  (Class|FourTaleCharacter|EquipWeapon (Variables|FourTale|GetCharacter))
  (Ability|EndAbility))