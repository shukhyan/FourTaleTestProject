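; GA_Fire is the gameplay ability that fires the character's current weapon.
; Activation starts the fire montage task and, without authority, sends the weapon's muzzle socket location through ServerFire; the authority branch does nothing.
; It then immediately commits and ends, also ending on montage interruption or cancellation, and OnEndAbility ends the montage task.
; The Server_Fire event passes a muzzle location to Fire.
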(event Custom|Server_Fire
  (params (MuzzleLocation :type Vector))
  (Class|FireGameplayAbility|Fire MuzzleLocation))

(event Ability|EventActivateAbility
  (bind _asynctaskproxy (|PlayMontageandWaitProxy "None" (Variables|FourTale|Montage|GetFireMontage) 1.0 "None" true 1.0 0.0 true)
    (:then
      (Variables|FourTale|Config|SetPlayMontageTask _asynctaskproxy)
      (Ability|HasAuthority
        (:True
          _)
        (:False
          (CallFunction|ServerFire (Class|FourTaleWeaponBase|GetMuzzleSocketLocation (Class|FireGameplayAbility|GetCurrentWeapon)))))
      (Ability|CommitAbility)
      (Ability|EndAbility))
    (:OnInterrupted
      (Ability|EndAbility :!label _label))
    (:OnCancelled
      (goto _label))))

(event Ability|EventOnEndAbility
  (params (bWasCancelled :type Boolean))
  (GameplayTasks|EndTask (Variables|FourTale|Config|GetPlayMontageTask)))